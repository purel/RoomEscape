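; Openable door actor that swings open and closed in response to its OnOpen and OnClose events.
; It caches its initial rotation at BeginPlay, and the DoorSwing timeline adds an animated yaw offset to it to rotate the whole actor.
; Closing plays the same timeline in reverse, and a timeline event track plays the lock sound at the door's location.
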(event OnClose(Door)
  (bind _openangle (Timeline|DoorSwing Reverse)
    (:Update
      (Transformation|SetActorRotation (Math|Rotator|CombineRotators (Math|Rotator|MakeRotator 0.0 0.0 _openangle) (Variables|Default|GetInitial%20Rotation))))
    (:DoorLockSound
      (Audio|PlaySoundatLocation "/Game/Audio/door-lock.door-lock" (Transformation|GetActorLocation)))))

(event OnOpen(Door)
  (bind _openangle (Timeline|DoorSwing Play)
    (:Update
      (Transformation|SetActorRotation (Math|Rotator|CombineRotators (Math|Rotator|MakeRotator 0.0 0.0 _openangle) (Variables|Default|GetInitial%20Rotation))))
    (:DoorLockSound
      (Audio|PlaySoundatLocation "/Game/Audio/door-lock.door-lock" (Transformation|GetActorLocation)))))

(event EventBeginPlay
  (Variables|Default|SetInitial%20Rotation (Transformation|GetActorRotation)))

(fn ConstructionScript)